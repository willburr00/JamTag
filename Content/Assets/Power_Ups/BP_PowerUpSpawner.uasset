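; BP_PowerUpSpawner periodically spawns power-up actors at random positions within a box-shaped area.
; On BeginPlay, a looping timer fires SpawnEvent every SpawnDelay seconds.
; Each spawn location is a random per-axis offset scaled by SpawnRange around SpawnCenter.
; A random four-way switch selects the spawn, but every branch currently leads to BP_Colorblind.
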(event Custom|SpawnEvent
  (switch int (Math|Random|RandomInteger 4)
    (:0
      _)
    (:1
      _)
    (:2
      _)
    (:3
      _))
  (Game|SpawnActorfromClass "/Game/Assets/Power_Ups/BP_Colorblind.BP_Colorblind_C" (Math|Transform|MakeTransform (+ (* (Math|Vector|MakeVector (Math|Random|RandomFloatinRange -1.0 1.0) (Math|Random|RandomFloatinRange -1.0 1.0) (Math|Random|RandomFloatinRange -1.0 1.0)) (Variables|Default|GetSpawnRange)) (Variables|Default|GetSpawnCenter))) "Undefined" 0 0))

(event EventBeginPlay
  (Utilities|Time|SetTimerbyEvent (delegate Custom|SpawnEvent) (Variables|Default|GetSpawnDelay) true))

(fn ConstructionScript)