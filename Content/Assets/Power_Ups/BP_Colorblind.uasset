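; Colorblind power-up pickup that afflicts every player except the one who collects it with a temporary colorblind effect.
; The first PlayableCharacter overlap passes a DoOnce, toggles the cube's visibility, prints a message and adds the effect to characters with other player IDs.
; After a five-second delay it gathers the characters again and removes the effect.
; The two colorblind query functions are unfinished, with their checks left unwired.
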(event OnComponentBeginOverlap(MyCollisionBox)
  (params (OverlappedComponent :type Primitive%20Component%20Object%20Reference) (OtherActor :type Actor%20Object%20Reference) (OtherComp :type Primitive%20Component%20Object%20Reference) (OtherBodyIndex :type Integer) (bFromSweep :type Boolean) (SweepResult :type Hit%20Result%20Structure%20%28by%20ref%29))
  ;[1 1 1] Consume if Used by Player
  (bind _asplayable_character (Utilities|Casting|CastToPlayableCharacter OtherActor))
  (Utilities|FlowControl|DoOnce false
    (:Completed
      (Rendering|ToggleVisibility (Variables|Default|GetCube) false)
      (Development|PrintString "Colorblind!")
      ;[1 1 1] Increment Players' Colorblind Effect
      (bind _outactors (Actor|GetAllActorsOfClass "/Script/GG_poop.PlayableCharacter"))
      (for _array_element _outactors
        (if (!= (Class|PlayableCharacter|GetPlayerID _array_element) (Class|PlayableCharacter|GetPlayerID _asplayable_character))
          (Class|PlayableCharacter|AddColorBlindEffect _array_element)))
      ;[1 1 1] Decrement Players' Colorblind Effect
      (Utilities|FlowControl|Delay 5.0)
      (bind _outactors_2 (Actor|GetAllActorsOfClass "/Script/GG_poop.PlayableCharacter"))
      (for _array_element_2 _outactors_2
        (if (!= (Class|PlayableCharacter|GetPlayerID _array_element_2) (Class|PlayableCharacter|GetPlayerID _asplayable_character))
          (Class|PlayableCharacter|RemoveColorBlindEffect _array_element_2))))))

(fn ConstructionScript)

(fn IsAnyPlayerColorblind
  (params (Players :type Array%20of%20Playable%20Character%20Object%20References))
  (for _array_element Players
    _)
  (return false))

(fn IsTilePlayerColorblind
  (params (Players :type Array%20of%20Playable%20Character%20Object%20References) (TriggerID :type Integer)))