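; BP_NeutralBomb is a single-use power-up that neutralises other players' tiles around it when a playable character overlaps it.
; The first valid overlap toggles the mesh's visibility, prints a message and scans all BP_triggerTile actors within Range.
; Tiles owned by a valid player other than the collector decrement that owner's tile count and switch TriggerID to the neutral value.
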(event OnComponentBeginOverlap(MyCollisionBox)
  (params (OverlappedComponent :type Primitive%20Component%20Object%20Reference) (OtherActor :type Actor%20Object%20Reference) (OtherComp :type Primitive%20Component%20Object%20Reference) (OtherBodyIndex :type Integer) (bFromSweep :type Boolean) (SweepResult :type Hit%20Result%20Structure%20%28by%20ref%29))
  ;[1 1 1] Consume if Used by Player
  (bind _asplayable_character (Utilities|Casting|CastToPlayableCharacter OtherActor))
  (Utilities|FlowControl|DoOnce false
    (:Completed
      (Rendering|ToggleVisibility (Variables|Default|GetStaticMesh) false)
      (Development|PrintString "Neutral Bomb!")
      ;[1 1 1] Check inside Range
      (bind _outactors (Actor|GetAllActorsOfClass "/Game/Assets/TriggerTiles/BP_triggerTile.BP_triggerTile_C"))
      (for _array_element _outactors
        (if (< (Transformation|GetDistanceTo _array_element) (Variables|Default|GetRange))
          ;[1 1 1] Check not Active or Neutral Player
          (if (and (< (Variables|/Game/Assets/TriggerTiles/BP_triggerTile.BP_triggerTile_C|GetTriggerID _array_element) 4) (!= (Variables|/Game/Assets/TriggerTiles/BP_triggerTile.BP_triggerTile_C|GetTriggerID _array_element) (Class|PlayableCharacter|GetPlayerID _asplayable_character)))
            ;[1 1 1] Tile Count --
            (Utilities|IsValid (Game|GetPlayerCharacter (Variables|/Game/Assets/TriggerTiles/BP_triggerTile.BP_triggerTile_C|GetTriggerID _array_element))
              (:Is%20Valid
                (bind _asplayable_character_2 (Utilities|Casting|CastToPlayableCharacter (Game|GetPlayerCharacter (Variables|/Game/Assets/TriggerTiles/BP_triggerTile.BP_triggerTile_C|GetTriggerID _array_element))))
                (Class|PlayableCharacter|RemovefromTileCount _asplayable_character_2 1)
                ;[1 1 1] Set Tile to Neutral
                (Variables|/Game/Assets/TriggerTiles/BP_triggerTile.BP_triggerTile_C|SetTriggerID _array_element 4)))))))))

(fn ConstructionScript)